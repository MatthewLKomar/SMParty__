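; Spline track Blueprint that moves a referenced ActorToMove along its spline in repeated runs.
; A timeline track scales the spline length into a distance, whose world location sets the actor's transform, and the timeline restarts after a short delay on finishing.
; Tick calls Play on alternate frames through a FlipFlop.
; Rotation derives from the world location vector rather than the spline's direction.
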(event EventBeginPlay)

(event Collision|EventActorBeginOverlap
  (params (OtherActor :type Actor%20Object%20Reference)))

(event EventTick
  (params (DeltaSeconds :type Float%20%28single-precision%29))
  (Utilities|FlowControl|FlipFlop
    (:A
      (bind _newtrack_0 (Timeline|Timeline_0 Play)
        (:Update
          (Transformation|SetActorTransform (Variables|Default|GetActorToMove) (Math|Transform|MakeTransform (Spline|GetLocationatDistanceAlongSpline (Variables|Default|GetSpline) (* (Spline|GetSplineLength (Variables|Default|GetSpline)) _newtrack_0) "World") (Math|Conversions|RotationFromXVector (Spline|GetLocationatDistanceAlongSpline (Variables|Default|GetSpline) (* (Spline|GetSplineLength (Variables|Default|GetSpline)) _newtrack_0) "World")))))
        (:Finished
          (Utilities|FlowControl|Delay 2.0)
          (Timeline|Timeline_0 PlayFromStart))))))

(fn ConstructionScript)