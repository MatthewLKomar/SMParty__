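; Light actor that strobes by switching its point light on and off at a regular interval.
; BeginPlay starts a looping timer at TimeBetweenStrobe that calls Strobe, where both FlipFlop branches make the same ToggleVisibility call on PointLight.
; It also saves the starting intensity in OldIntensity, which nothing here reads, and a delayed Strobe call is left unconnected.
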(event EventBeginPlay
  (Variables|Default|SetOldIntensity (Variables|/Script/Engine.LightComponentBase|GetIntensity (Variables|Default|GetPointLight)))
  (Utilities|Time|SetTimerbyFunctionName 0 "Strobe" (Variables|Default|GetTimeBetweenStrobe) true))

(event EventTick
  (params (DeltaSeconds :type Float%20%28single-precision%29)))

(fn ConstructionScript
  (|CallParentFunction))

(fn Strobe
  (Utilities|FlowControl|FlipFlop
    (:A
      (Rendering|ToggleVisibility (Variables|Default|GetPointLight) false))
    (:B
      (Rendering|ToggleVisibility (Variables|Default|GetPointLight) false))))